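; BPC_SCORE is a score component that keeps a running score and shows it on the player's HUD.
; Scoretoadd adds to the score, while Scoretotakeaway sets it to the passed amount minus the current score, in that operand order, clamped at zero and a large maximum.
; Both then call Updateuiscore, which casts the player character to BP_ThirdPersonCharacter and sends the score as text to its HUD widget.
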(fn `Scoretoadd`
  (params (ScoretoAdd :type Integer))
  (set `self.Score` (+ ScoretoAdd (`self.Score`)))
  (`self.updateuiscore`))

(fn `Scoretotakeaway`
  (params (scoretotakeaway :type Integer))
  (set `self.Score` (`KismetMathLibrary.Clamp` (- scoretotakeaway (`self.Score`)) 0 232343252))
  (`self.updateuiscore`))

(fn `updateuiscore`
  (bind _asbp_third_person_character (cast `/Game/ThirdPerson/Blueprints/BP_ThirdPersonCharacter` (`GameplayStatics.GetPlayerCharacter` 0)))
  (`/Game/UI/wbp_HUD.UpdateUI` (`/Game/ThirdPerson/Blueprints/BP_ThirdPersonCharacter.wbp_HUD_ref` _asbp_third_person_character) (`KismetTextLibrary.Conv_IntToText` (`self.Score`))))