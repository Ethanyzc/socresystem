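; BPM_collerctor is a pickup actor that either adds to or takes away from the player's score when touched.
; A sphere overlap casts to BP_ThirdPersonCharacter and passes Reward to its BPCSCORE component, subtracting when Hazard is set and adding otherwise, then destroys itself.
; The construction script applies the Collectabemesh variable to the static mesh, so each instance can have its own look.
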(event `self.Sphere.OnComponentBeginOverlap`
  (params (OverlappedComponent :type "PrimitiveComponent Object Reference") (OtherActor :type "Actor Object Reference") (OtherComp :type "PrimitiveComponent Object Reference") (OtherBodyIndex :type Integer) (bFromSweep :type Boolean) (SweepResult :type "HitResult Structure (by ref)"))
  (bind _asbp_third_person_character (cast `/Game/ThirdPerson/Blueprints/BP_ThirdPersonCharacter` OtherActor))
  (if (`self.hazard`)
    (bind _bpc_score (`/Game/ThirdPerson/Blueprints/BP_ThirdPersonCharacter.BPC_SCORE` _asbp_third_person_character))
    (`/Game/blueprint/components/BPC_SCORE.Scoretotakeaway` _bpc_score (`self.Reward`))
    (else
      (`/Game/blueprint/components/BPC_SCORE.Scoretoadd` _bpc_score (`self.Reward`))))
  (`self.K2_DestroyActor`))

(fn `UserConstructionScript`
  (`StaticMeshComponent.SetStaticMesh` (`self.StaticMesh`) (`self.collectabemesh`)))